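; BP_Tooltip_LookOn is a tooltip actor whose text turns to face the player's camera while a character is nearby.
; It extends a parent Blueprint, setting a LookAt flag on overlap when CharacterInBox is valid and clearing it on any end overlap.
; Each tick, while the flag is set, it rotates TooltipText toward the FollowCamera of BP_ThirdPersonCharacter using a look-at rotation.
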(event `self.ReceiveTick`
  (params (DeltaSeconds :type "Float (single-precision)"))
  (`parent.ReceiveTick` DeltaSeconds)
  (`self.LookingAtPlayerCamera`))

(event `self.ReceiveActorBeginOverlap`
  (params (OtherActor :type "Actor Object Reference"))
  (`parent.ReceiveActorBeginOverlap` OtherActor)
  (`self.CharacterInBox`
    (:`then`
      (set `self.LookAt` true))
    (:`else`)))

(event `self.ReceiveActorEndOverlap`
  (params (OtherActor :type "Actor Object Reference"))
  (`parent.ReceiveActorEndOverlap` OtherActor)
  (set `self.LookAt` false))

(fn `LookingAtPlayerCamera`
  (locals (L_CameraLocation :type "Vector Structure" :default (0.0 0.0 0.0)))
  (if (`self.LookAt`)
    (bind _characterinbox (`self.CharacterInBox`)
      (:`then`
        (bind _asbp_third_person_character (cast `/Game/Blueprints/Characters/BP_ThirdPersonCharacter` _characterinbox))
        (set `local.L_CameraLocation` (`SceneComponent.K2_GetComponentLocation` (`/Game/Blueprints/Characters/BP_ThirdPersonCharacter.FollowCamera` _asbp_third_person_character)))
        (`SceneComponent.K2_SetWorldRotation` (`self.TooltipText`) (`KismetMathLibrary.FindLookAtRotation` (`SceneComponent.K2_GetComponentLocation` (`self.TooltipText`)) (`local.L_CameraLocation`)) false false))
      (:`else`))))

(fn `UserConstructionScript`
  (`parent.UserConstructionScript`))