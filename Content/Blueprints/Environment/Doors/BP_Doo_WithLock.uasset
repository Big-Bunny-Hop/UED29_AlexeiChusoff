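; Lockable child door Blueprint that opens only while unlocked and shows its lock state with a red or green point light.
; Interact toggles an unlocked door, or checks the overlapped actor's BP_BackpackComponent for required quest keys and unlocks once all are found.
; Matched keys are removed during the check, even if others are missing.
; SwitchLock, Lock and Unlock change the state directly, though Lock only affects doors without required keys.
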(event `self.OpenDoor`
  (if (not (`self.IsDoorLocked`))
    (`parent.OpenDoor`)))

(event `self.CloseDoor`
  (`parent.CloseDoor`))

(fn `Interact`
  (returns (Success :type Boolean))
  (locals (L_Backpack :type "/Game/Blueprints/Components/BP_BackpackComponent Object Reference") (L_ItemInrement :type Integer) (L_ItemName :type Name))
  (if (`self.IsReadyToInteract`)
    (if (not (`self.IsDoorLocked`))
      (if (`self.IsOpen`)
        (`self.CloseDoor`)
        (return true)
        (else
          (`self.OpenDoor`)
          (return true)))
      (elif (`KismetArrayLibrary.Array_IsValidIndex` (`self.NeededKeysName`))
        (bind _overlappedactor (`self.OverlappedActor`)
          (:`then`
            (bind _returnvalue (`self.GetComponentByClass` _overlappedactor "/Game/Blueprints/Components/BP_BackpackComponent.BP_BackpackComponent_C"))
            (`/Engine/EditorBlueprintResources/StandardMacros.IsValid` _returnvalue
              (:`Is Valid`
                (set `local.L_Backpack` _returnvalue)
                (for _array_element (`self.NeededKeysName`)
                  (set `local.L_ItemName` _array_element)
                  (if (`BlueprintSetLibrary.Set_Contains` (`/Game/Blueprints/Components/BP_BackpackComponent.QuestItems` (`local.L_Backpack`)) (`local.L_ItemName`))
                    (`/Engine/EditorBlueprintResources/StandardMacros.IncrementInt` (`local.L_ItemInrement`)
                      (:`  `
                        ;[0.2222 0.9002 1] Remove item from inventory after use
                        (`/Game/Blueprints/Components/BP_BackpackComponent.RemoveQuestItem` (`local.L_Backpack`) (`local.L_ItemName`))))))
                (if (== (`local.L_ItemInrement`) (`KismetArrayLibrary.Array_Length` (`self.NeededKeysName`)))
                  (`self.Unlock`)
                  (else
                    (return true))))
              (:`Is Not Valid`
                (return true))))
          (:`else`
            (return true)))
        (else
          (return true))))
    (else
      (return false))))

(fn `Lock`
  (if (not (`KismetArrayLibrary.Array_IsValidIndex` (`self.NeededKeysName`)))
    (set `self.IsDoorLocked` true)
    (`self.UpdateDoorLockIndication`)))

(fn `SwitchLock`
  (set `self.IsDoorLocked` (not (`self.IsDoorLocked`)))
  (`self.UpdateDoorLockIndication`))

(fn `Unlock`
  (set `self.IsDoorLocked` false)
  (`self.UpdateDoorLockIndication`))

(fn `UpdateDoorLockIndication`
  (`LightComponent.SetLightColor` (`self.PointLightLockIndicator`) (`KismetMathLibrary.SelectColor` (struct :`R` 1.0 :`A` 1.0) (struct :`G` 1.0 :`B` 0.054357 :`A` 1.0) (`self.IsDoorLocked`)) true))

(fn `UserConstructionScript`
  (`parent.UserConstructionScript`)
  (`self.UpdateDoorLockIndication`))